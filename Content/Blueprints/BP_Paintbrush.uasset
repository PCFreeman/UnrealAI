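; BP_Paintbrush is a colour-matched switch that the player (BP_Kuutio) charges to move linked actors.
; While an overlapping player's active colour matches, Tick drains their ability in timed thirds, raising the brush's charge and material blend.
; At full charge, Action lerps MovingActors on a timeline to temporary scene components placed from brush-relative MovingDest transforms, optionally changing location only.
; Construction tints the brush from DT_Colour_Info and adjusts the MovingDest array.
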(event EventTick
  (params (DeltaSeconds :type Float%20%28single-precision%29))
  (if (not (Variables|Default|Getactivated))
    ;[1 1 1] Update how coloured I am, dependent to how charged I am.
    (Rendering|Material|SetScalarParameterValue (Variables|Default|GetmyMaterial) "blend" (Variables|Default|GetcurrentCharge) :!class /Script/Engine.MaterialInstanceDynamic)
    (if (not (Variables|Default|Getdraining))
      (if (Variables|Default|GetinRange)
        (bind _asbp_kuutio (Utilities|Casting|CastToBP_Kuutio (Variables|Default|GetplayerRef)))
        (if (Utilities|Enum|Equal(Enum) (Variables|/Game/Kuutio/BP_Kuutio.BP_Kuutio_C|GetactiveColour _asbp_kuutio) (Variables|Default|GetmyColour))
          (Variables|Default|Setdraining true)
          (bind _returnvalue (Audio|SpawnSoundatLocation "/Game/Audio/S_Brush.S_Brush" (Transformation|GetActorLocation) "0, 0, 0" 1.0 1.0 0.0 0 0))
          (Variables|Default|SetsoundRef _returnvalue)
          (Variables|/Game/Kuutio/BP_Kuutio.BP_Kuutio_C|SetactiveAbilityRemaining _asbp_kuutio (- (Variables|/Game/Kuutio/BP_Kuutio.BP_Kuutio_C|GetactiveAbilityRemaining _asbp_kuutio) 0.33))
          (bind _output_get (Variables|Default|SetcurrentCharge (+ (Variables|Default|GetcurrentCharge) 0.33)))
          (if (Math|Float|NearlyEqual(Float) _output_get 1.0 0.1)
            (Rendering|Material|SetScalarParameterValue (Variables|Default|GetmyMaterial) "blend" 1.0 :!class /Script/Engine.MaterialInstanceDynamic)
            (Variables|Default|Setactivated true)
            (Utilities|FlowControl|Delay 1.0)
            (Variables|Default|Setdraining false)
            (Audio|Components|Audio|Stop (Variables|Default|GetsoundRef))
            (Audio|PlaySound2D "/Game/Audio/S_Activate.S_Activate" 1.0 1.0 0.0 0 0)
            (CallFunction|Action)
            (else
              (Utilities|FlowControl|Delay 1.0)
              (Variables|Default|Setdraining false)
              (Audio|Components|Audio|Stop (Variables|Default|GetsoundRef)))))))))

(event OnComponentBeginOverlap(Collision)
  (params (OverlappedComponent :type Primitive%20Component%20Object%20Reference) (OtherActor :type Actor%20Object%20Reference) (OtherComp :type Primitive%20Component%20Object%20Reference) (OtherBodyIndex :type Integer) (bFromSweep :type Boolean) (SweepResult :type Hit%20Result%20Structure%20%28by%20ref%29))
  ;[1 1 1] Boolean is true and store reference if contacted actor is player.
  (if (Actor|ActorHasTag OtherActor "Player")
    (Variables|Default|SetplayerRef OtherActor)
    (Variables|Default|SetinRange true)))

(event OnComponentEndOverlap(Collision)
  (params (OverlappedComponent :type Primitive%20Component%20Object%20Reference) (OtherActor :type Actor%20Object%20Reference) (OtherComp :type Primitive%20Component%20Object%20Reference) (OtherBodyIndex :type Integer))
  ;[1 1 1] Boolean is false when the player leaves the overlap area.
  (if (Actor|ActorHasTag OtherActor "Player")
    (Variables|Default|SetinRange false)))

(event Custom|Action
  (Utilities|FlowControl|Sequence
    (:then_0
      (for _array_element (Variables|Default|GetMovingActors)
        (Utilities|Array|Add (Variables|Default|GetorigLocations) (Transformation|GetActorTransform _array_element))))
    (:then_1
      (for _array_element_2 (Variables|DONOTEDIT|GetMovingDest)
        (bind _returnvalue (AddComponent|AddSceneComponent false _array_element_2))
        (Utilities|Array|Add (Variables|DONOTEDIT|GetmovingDestinationComponents) _returnvalue)))
    (:then_2
      (bind _delta (Timeline|Timeline_0 PlayFromStart)
        (:Update
          (for (_array_element_3 _array_index) (Variables|Default|GetMovingActors)
            (if (Variables|Default|GetfinallDestinationChange)
              (Transformation|SetActorTransform _array_element_3 (Math|Transform|Lerp(Transform) (Math|Transform|MakeTransform (.location (Utilities|Array|Get(acopy) (Variables|Default|GetorigLocations) _array_index)) (.rotation (Utilities|Array|Get(acopy) (Variables|Default|GetorigLocations) _array_index)) (.scale (Utilities|Array|Get(acopy) (Variables|Default|GetorigLocations) _array_index))) (Math|Transform|MakeTransform (.location (Transformation|GetWorldTransform (Utilities|Array|Get(acopy) (Variables|DONOTEDIT|GetmovingDestinationComponents) _array_index))) (.rotation (Utilities|Array|Get(acopy) (Variables|Default|GetorigLocations) _array_index)) (.scale (Utilities|Array|Get(acopy) (Variables|Default|GetorigLocations) _array_index))) _delta))
              (else
                (Transformation|SetActorTransform _array_element_3 (Math|Transform|Lerp(Transform) (Math|Transform|MakeTransform (.location (Utilities|Array|Get(acopy) (Variables|Default|GetorigLocations) _array_index)) (.rotation (Utilities|Array|Get(acopy) (Variables|Default|GetorigLocations) _array_index)) (.scale (Utilities|Array|Get(acopy) (Variables|Default|GetorigLocations) _array_index))) (Math|Transform|MakeTransform (.location (Transformation|GetWorldTransform (Utilities|Array|Get(acopy) (Variables|DONOTEDIT|GetmovingDestinationComponents) _array_index))) (.rotation (Transformation|GetWorldTransform (Utilities|Array|Get(acopy) (Variables|DONOTEDIT|GetmovingDestinationComponents) _array_index))) (.scale (Transformation|GetWorldTransform (Utilities|Array|Get(acopy) (Variables|DONOTEDIT|GetmovingDestinationComponents) _array_index)))) _delta))))))
        (:Finished
          (for _array_element_4 (Variables|DONOTEDIT|GetmovingDestinationComponents)
            (Components|DestroyComponent _array_element_4)))))))

(fn ConstructionScript
  (Utilities|FlowControl|Sequence
    (:then_0
      (bind _returnvalue (Utilities|GetDataTableRow "/Game/Blueprints/DT_Colour_Info.DT_Colour_Info" (Utilities|String|StringToName (Utilities|String|EnumtoString (Variables|Default|GetmyColour))))
        (:then
          (bind _returnvalue_2 (Rendering|Material|CreateDynamicMaterialInstance "/Game/Art/Materials/M_Brush.M_Brush" "None" :!class /Script/Engine.KismetMaterialLibrary))
          (bind _output_get (Variables|Default|SetmyMaterial _returnvalue_2))
          (Rendering|Material|SetVectorParameterValue _output_get "secondaryColour" (.Colour (Utilities|Struct|BreakST_Colour_Info _returnvalue)) :!class /Script/Engine.MaterialInstanceDynamic)
          (Rendering|Material|SetMaterial (Variables|Default|GetBrush) 0 _output_get))))
    (:then_1
      (if (< (Utilities|Array|Length (Variables|DONOTEDIT|GetMovingDest)) (Utilities|Array|Length (Variables|Default|GetMovingActors)))
        (for _array_element (Variables|Default|GetMovingActors)
          (if (Utilities|IsValid _array_element)
            (Utilities|Array|Add (Variables|DONOTEDIT|GetMovingDest) (Math|Transform|MakeTransform "0, 0,500.000000" "0, 0, 0" "1,1,1"))))
        (elif (> (Utilities|Array|Length (Variables|DONOTEDIT|GetMovingDest)) (Utilities|Array|Length (Variables|Default|GetMovingActors)))
          (Utilities|Array|Resize (Variables|DONOTEDIT|GetMovingDest) (Utilities|Array|Length (Variables|Default|GetMovingActors))))))))
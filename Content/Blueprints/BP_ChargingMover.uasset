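; Charging platform that, once activated by the player, moves linked actors such as doors to set destinations.
; While the player overlaps it at or above minimum speed, charge builds toward a platform-length-based threshold, blending its colour toward yellow; slowing or leaving resets it, while blinking activates it instantly.
; Activation plays a sound and a timeline lerps MovingActors toward temporary scene components built from MovingDest, which the construction script auto-sizes.
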(event EventBeginPlay
  (bind _charging_platform (Variables|Default|GetCharging_Platform))
  (bind _returnvalue (Transformation|GetWorldScale _charging_platform))
  ;[1 1 1] Determine range of acceptable active times dependent on length of charging platform
  (Variables|Default|SetmaximumCharge (* (.x _returnvalue) 0.125))
  (Variables|Default|SetminimumCharge (* (.x _returnvalue) 0.083))
  ;[1 1 1] Then, force scale of non-calculated components to default.
  (Transformation|SetRelativeScale3D (Variables|Default|GetCharging_Platform) (Math|Vector|MakeVector (.x _returnvalue) 4.0 0.15))
  (Transformation|SetRelativeScale3D (Variables|Default|GetDefaultSceneRoot) (Math|Vector|MakeVector 1.0 1.0 1.0))
  (Transformation|SetActorScale3D self "1.000000,1.000000,1.000000"))

(event EventTick
  (params (DeltaSeconds :type Float%20%28single-precision%29))
  (bind _playerref (Variables|Default|GetplayerRef))
  ;[1 1 1] If I am inactive and player is inrange...
  (if (not (Variables|Default|Getactivated))
    ;;[1 1 1] Update how coloured I am, dependent to how charged I am.
    (Rendering|Material|SetScalarParameterValue (Variables|Default|GetmyMaterial) "blend" (/ (Variables|Default|GetcurrentCharge) (Variables|Default|GetminimumCharge)) :!class /Script/Engine.MaterialInstanceDynamic)
    (if (Variables|Default|GetinRange)
      ;[1 1 1] If player is blinking, skip charge sequence
      (bind _asbp_kuutio (Utilities|Casting|CastToBP_Kuutio _playerref))
      (if (Variables|/Game/Kuutio/BP_Kuutio.BP_Kuutio_C|Getblinking _asbp_kuutio)
        ;[1 1 1] If player has created charge within the acceptable limits, open door.
        (Variables|Default|Setactivated true :!label _label)
        (Rendering|Material|SetScalarParameterValue (Variables|Default|GetmyMaterial) "blend" 1.0 :!class /Script/Engine.MaterialInstanceDynamic)
        (Audio|PlaySound2D "/Game/Audio/S_Activate.S_Activate" 1.0 1.0 0.0 0 0)
        (CallFunction|DoorEleveting)
        (else
          ;[1 1 1] If player is at adequete speed, build charge. Otherwise, reset charge.
          (if (>= (Math|Vector|VectorLength (Transformation|GetVelocity _playerref)) (Variables|Default|GetminSpeed))
            (Variables|Default|SetcurrentCharge (+ DeltaSeconds (Variables|Default|GetcurrentCharge)))
            (if (Math|Float|InRange(Float) (Variables|Default|GetcurrentCharge) (Variables|Default|GetminimumCharge) (Variables|Default|GetmaximumCharge))
              (goto _label))
            (else
              (Variables|Default|SetcurrentCharge 0.0 :!label _label_2)))))
      (else
        (goto _label_2)))))

(event OnComponentBeginOverlap(Charging_Platform_Collision)
  (params (OverlappedComponent :type Primitive%20Component%20Object%20Reference) (OtherActor :type Actor%20Object%20Reference) (OtherComp :type Primitive%20Component%20Object%20Reference) (OtherBodyIndex :type Integer) (bFromSweep :type Boolean) (SweepResult :type Hit%20Result%20Structure%20%28by%20ref%29))
  ;[1 1 1] Boolean is true and store reference if contacted actor is player.
  (if (Actor|ActorHasTag OtherActor "Player")
    (Variables|Default|SetplayerRef OtherActor)
    (Variables|Default|SetinRange true)))

(event OnComponentEndOverlap(Charging_Platform_Collision)
  (params (OverlappedComponent :type Primitive%20Component%20Object%20Reference) (OtherActor :type Actor%20Object%20Reference) (OtherComp :type Primitive%20Component%20Object%20Reference) (OtherBodyIndex :type Integer))
  ;[1 1 1] Boolean is false when the player leaves the overlap area.
  (if (Actor|ActorHasTag OtherActor "Player")
    (Variables|Default|SetinRange false)))

(event Custom|Door_Eleveting
  (Utilities|FlowControl|Sequence
    (:then_0
      (for _array_element (Variables|Default|GetMovingActors)
        (Utilities|Array|Add (Variables|Default|GetorigLocations) (Transformation|GetActorTransform _array_element))))
    (:then_1
      (for _array_element_2 (Variables|DONOTEDIT|GetMovingDest)
        (bind _returnvalue (AddComponent|AddSceneComponent false _array_element_2))
        (Utilities|Array|Add (Variables|DONOTEDIT|GetmovingDestinationComponents) _returnvalue)))
    (:then_2
      (bind _delta (Timeline|Timeline_0 PlayFromStart)
        (:Update
          (for (_array_element_3 _array_index) (Variables|Default|GetMovingActors)
            (if (Variables|Default|GetfinallDestinationChange)
              (Transformation|SetActorTransform _array_element_3 (Math|Transform|Lerp(Transform) (Math|Transform|MakeTransform (.location (Utilities|Array|Get(acopy) (Variables|Default|GetorigLocations) _array_index)) (.rotation (Utilities|Array|Get(acopy) (Variables|Default|GetorigLocations) _array_index)) (.scale (Utilities|Array|Get(acopy) (Variables|Default|GetorigLocations) _array_index))) (Math|Transform|MakeTransform (.location (Transformation|GetWorldTransform (Utilities|Array|Get(acopy) (Variables|DONOTEDIT|GetmovingDestinationComponents) _array_index))) (.rotation (Utilities|Array|Get(acopy) (Variables|Default|GetorigLocations) _array_index)) (.scale (Utilities|Array|Get(acopy) (Variables|Default|GetorigLocations) _array_index))) _delta))
              (else
                (Transformation|SetActorTransform _array_element_3 (Math|Transform|Lerp(Transform) (Math|Transform|MakeTransform (.location (Utilities|Array|Get(acopy) (Variables|Default|GetorigLocations) _array_index)) (.rotation (Utilities|Array|Get(acopy) (Variables|Default|GetorigLocations) _array_index)) (.scale (Utilities|Array|Get(acopy) (Variables|Default|GetorigLocations) _array_index))) (Math|Transform|MakeTransform (.location (Transformation|GetWorldTransform (Utilities|Array|Get(acopy) (Variables|DONOTEDIT|GetmovingDestinationComponents) _array_index))) (.rotation (Transformation|GetWorldTransform (Utilities|Array|Get(acopy) (Variables|DONOTEDIT|GetmovingDestinationComponents) _array_index))) (.scale (Transformation|GetWorldTransform (Utilities|Array|Get(acopy) (Variables|DONOTEDIT|GetmovingDestinationComponents) _array_index)))) _delta))))))
        (:Finished
          (for _array_element_4 (Variables|DONOTEDIT|GetmovingDestinationComponents)
            (Components|DestroyComponent _array_element_4)))))))

(fn ConstructionScript
  (Utilities|FlowControl|Sequence
    (:then_0
      (bind _returnvalue (Utilities|GetDataTableRow "/Game/Blueprints/DT_Colour_Info.DT_Colour_Info" "Uncoloured")
        (:then
          (bind _returnvalue_2 (Rendering|Material|CreateDynamicMaterialInstance "/Game/Art/Materials/M_Colour.M_Colour" "None" :!class /Script/Engine.KismetMaterialLibrary))
          (bind _output_get (Variables|Default|SetmyMaterial _returnvalue_2))
          (Rendering|Material|SetVectorParameterValue _output_get "baseColour" (.Colour (Utilities|Struct|BreakST_Colour_Info _returnvalue)) :!class /Script/Engine.MaterialInstanceDynamic)
          (bind _returnvalue_3 (Utilities|GetDataTableRow "/Game/Blueprints/DT_Colour_Info.DT_Colour_Info" "Yellow")
            (:then
              (Rendering|Material|SetVectorParameterValue (Variables|Default|GetmyMaterial) "secondaryColour" (.Colour (Utilities|Struct|BreakST_Colour_Info _returnvalue_3)) :!class /Script/Engine.MaterialInstanceDynamic)
              (Rendering|Material|SetMaterial (Variables|Default|GetCharging_Platform) 0 _output_get))))))
    (:then_1
      (if (< (Utilities|Array|Length (Variables|DONOTEDIT|GetMovingDest)) (Utilities|Array|Length (Variables|Default|GetMovingActors)))
        (for _array_element (Variables|Default|GetMovingActors)
          (if (Utilities|IsValid _array_element)
            (Utilities|Array|Add (Variables|DONOTEDIT|GetMovingDest) (Math|Transform|MakeTransform "0, 0,500.000000" "0, 0, 0" "1,1,1"))))
        (elif (> (Utilities|Array|Length (Variables|DONOTEDIT|GetMovingDest)) (Utilities|Array|Length (Variables|Default|GetMovingActors)))
          (Utilities|Array|Resize (Variables|DONOTEDIT|GetMovingDest) (Utilities|Array|Length (Variables|Default|GetMovingActors))))))))
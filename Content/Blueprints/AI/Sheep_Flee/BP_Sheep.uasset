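; BP_Sheep is a sheep AI that wanders the navmesh and flees from the player.
; Entering the inner Range volume sets IsFeared, and only leaving the LargeRange volume clears it, giving hysteresis.
; Tick chooses between Flee, which moves to a point a short step directly away from the player, and Roam, which moves to random nearby navigable points after a delay.
; Damage from the player only prints a debug string.
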(event OnComponentEndOverlap(largeRange)
  (params (OverlappedComponent :type Primitive%20Component%20Object%20Reference) (OtherActor :type Actor%20Object%20Reference) (OtherComp :type Primitive%20Component%20Object%20Reference) (OtherBodyIndex :type Integer))
  (if (Actor|ActorHasTag OtherActor "Player")
    (Variables|Default|SetIsFeared false)))

(event OnComponentBeginOverlap(Range)
  (params (OverlappedComponent :type Primitive%20Component%20Object%20Reference) (OtherActor :type Actor%20Object%20Reference) (OtherComp :type Primitive%20Component%20Object%20Reference) (OtherBodyIndex :type Integer) (bFromSweep :type Boolean) (SweepResult :type Hit%20Result%20Structure%20%28by%20ref%29))
  (if (Actor|ActorHasTag OtherActor "Player")
    (Variables|Default|SetIsFeared true)))

(event OnComponentEndOverlap(Range)
  (params (OverlappedComponent :type Primitive%20Component%20Object%20Reference) (OtherActor :type Actor%20Object%20Reference) (OtherComp :type Primitive%20Component%20Object%20Reference) (OtherBodyIndex :type Integer))
  (if (Actor|ActorHasTag OtherActor "Player")
    _))

(event Game|Damage|EventAnyDamage
  (params (Damage :type Float%20%28single-precision%29) (DamageType :type Damage%20Type%20Object%20Reference) (InstigatedBy :type Controller%20Object%20Reference) (DamageCauser :type Actor%20Object%20Reference))
  (if (== InstigatedBy (Game|GetPlayerController 0))
    (Development|PrintString "Off")))

(event EventTick
  (params (DeltaSeconds :type Float%20%28single-precision%29))
  ;[1 1 1] If I'm not targeting the player (they are not within pawnsensing range)
  (if (Variables|Default|GetIsFeared)
    (CallFunction|Flee)
    (else
      (CallFunction|Roam))))

(event Custom|Roam
  (Utilities|FlowControl|Delay 2.0)
  (AI|AIMoveTo (Class|PawnMovementComponent|GetPawnOwner (Variables|Character|GetCharacterMovement)) (.RandomLocation (Class|NavigationSystemV1|GetRandomPointinNavigableRadius (Transformation|GetActorLocation) 5e+02 0 "/Script/AIModule.NavFilter_AIControllerDefault")) 0 5.0 false))

(event Custom|Flee
  (bind _returnvalue (Game|GetPlayerCharacter 0))
  (bind _returnvalue_2 (Transformation|GetActorLocation))
  (bind _returnvalue_3 (Transformation|GetActorLocation _returnvalue))
  (bind _returnvalue_4 (Math|Rotator|FindLookatRotation _returnvalue_2 _returnvalue_3))
  (bind _returnvalue_5 (Math|Vector|GetForwardVector _returnvalue_4))
  (bind _returnvalue_6 (* _returnvalue_5 -5e+01))
  (bind _returnvalue_7 (+ _returnvalue_2 _returnvalue_6))
  (bind (_x _y) (Math|Vector|BreakVector _returnvalue_7))
  (AI|AIMoveTo (Class|PawnMovementComponent|GetPawnOwner (Variables|Character|GetCharacterMovement)) (Math|Vector|MakeVector _x _y (.Z (Math|Vector|BreakVector _returnvalue_2))) 0 0.0 false))

(fn ConstructionScript)
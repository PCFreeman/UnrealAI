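; BP_Cleanser is a water-bound creature that calls ResetToDefault on any BP_Kuutio, the player, that enters its sphere.
; Overlapping BP_Water sets its home water and an in-water flag.
; Tick uses that flag to raise or lower a clamped water level over ten seconds, scaling the actor between quarter and full size.
; Chase-and-return AI movement exists but is disconnected, leaving the PawnSensing event empty.
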(event OnComponentBeginOverlap(Sphere)
  (params (OverlappedComponent :type Primitive%20Component%20Object%20Reference) (OtherActor :type Actor%20Object%20Reference) (OtherComp :type Primitive%20Component%20Object%20Reference) (OtherBodyIndex :type Integer) (bFromSweep :type Boolean) (SweepResult :type Hit%20Result%20Structure%20%28by%20ref%29))
  (bind _asbp_kuutio (Utilities|Casting|CastToBP_Kuutio OtherActor))
  (Default|ResettoDefault _asbp_kuutio))

(event OnSeePawn(PawnSensing)
  (params (Pawn :type Pawn%20Object%20Reference)))

(event Collision|EventActorEndOverlap
  (params (OtherActor :type Actor%20Object%20Reference))
  (Utilities|Casting|CastToBP_Water OtherActor)
  (Variables|Default|SetinWater false))

(event EventTick
  (params (DeltaSeconds :type Float%20%28single-precision%29))
  (bind _returnvalue (/ DeltaSeconds 1e+01))
  (if (Variables|Default|GetinWater)
    (Variables|Default|SetwaterPercent (Math|Float|Clamp(Float) (+ (Variables|Default|GetwaterPercent) _returnvalue)))
    (else
      (Variables|Default|SetwaterPercent (Math|Float|Clamp(Float) (- (Variables|Default|GetwaterPercent) _returnvalue)))))
  (Transformation|SetActorScale3D (Math|Vector|Lerp(Vector) "0.250000,0.250000,0.250000" "1.000000,1.000000,1.000000" (Variables|Default|GetwaterPercent))))

(event Collision|EventActorBeginOverlap
  (params (OtherActor :type Actor%20Object%20Reference))
  (bind _asbp_water (Utilities|Casting|CastToBP_Water OtherActor))
  (Variables|Default|SethomeWaterRef _asbp_water)
  (Variables|Default|SetinWater true))

(fn ConstructionScript)
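; BP_Slurper is an enemy AI that drains the player's (BP_Kuutio) active colour ability on contact.
; It roams random navigable points, chasing the player via PawnSensing while thirsty, with a retriggerable delay clearing the target.
; Slurping copies the player's colour through DT_Colour_Info and reduces ability charge and slurp count, while absorbing turpentine kills it.
; Hits from a damage-capable player kill it, spawning a one-use BP_Paint_Dish of its colour unless uncoloured.
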(event EventTick
  (params (DeltaSeconds :type Float%20%28single-precision%29))
  ;[1 1 1] If I'm not targeting the player (they are not within pawnsensing range), then roam
  (Utilities|FlowControl|Delay 2.0)
  (if (not (Variables|Default|GetisTargetingPlayer))
    (AI|AIMoveTo (AI|GetAIController self) (.RandomLocation (Class|NavigationSystemV1|GetRandomPointinNavigableRadius (Transformation|GetActorLocation) 5e+02 0 0)) 0 -1.0 "Default" "Default" true true)))

(event OnSeePawn(PawnSensing)
  (params (Pawn :type Pawn%20Object%20Reference))
  ;[1 1 1] If I see the player and I'm still thirsty...
  (bind _asbp_kuutio (Utilities|Casting|CastToBP_Kuutio Pawn)
    (:then
      (if (Variables|Default|Getthirsty)
        ;[1 1 1] I tell my controller to move me towards the player
        (AI|Navigation|MovetoActor (AI|GetAIController self) _asbp_kuutio 0.0 true true true 0)
        (Variables|Default|SetisTargetingPlayer true)))
    (:CastFailed
      _))
  ;[1 1 1] Then if PawnSensing does not refire, I can no longer see the player.
  (Utilities|FlowControl|RetriggerableDelay 0.6)
  (Variables|Default|SetisTargetingPlayer false))

(event Collision|EventHit
  (params (MyComp :type Primitive%20Component%20Object%20Reference) (Other :type Actor%20Object%20Reference) (OtherComp :type Primitive%20Component%20Object%20Reference) (bSelfMoved :type Boolean) (HitLocation :type Vector :default "0, 0, 0") (HitNormal :type Vector :default "0, 0, 0") (NormalImpulse :type Vector :default "0, 0, 0") (Hit :type Hit%20Result%20Structure%20%28by%20ref%29))
  (bind _returnvalue (Transformation|GetActorTransform))
  (bind _asbp_kuutio (Utilities|Casting|CastToBP_Kuutio Other))
  (if (Variables|/Game/Kuutio/BP_Kuutio.BP_Kuutio_C|GetcanDamage _asbp_kuutio)
    (Audio|PlaySoundatLocation "/Game/Audio/S_AIDeath.S_AIDeath" (Transformation|GetActorLocation) "0, 0, 0" 1.0 1.0 0.0 0 0 0)
    (if (not (Variables|Default|GetisDying))
      (Variables|Default|SetisDying true)
      ;[1 1 1] Die after 2s, and then if I'm not uncoloured...
      (Actor|SetLifeSpan 2.0)
      (Utilities|FlowControl|Delay 1.0)
      (if (Utilities|Enum|NotEqual(Enum) (Variables|Default|GetmyColour) "NewEnumerator9")
        ;[1 1 1] ...spawn and colour an appropriate, one-time use paint dish.
        (bind _returnvalue_2 (Game|SpawnActorfromClass "/Game/Blueprints/BP_Paint_Dish.BP_Paint_Dish_C" (Math|Transform|MakeTransform (Math|Vector|MakeVector (.x (.location _returnvalue)) (.y (.location _returnvalue)) (- (.z (.location _returnvalue)) 5e+01)) (.rotation _returnvalue) (.scale _returnvalue)) "Undefined" 0 0))
        (bind _output_get (Variables|/Game/Blueprints/BP_Paint_Dish.BP_Paint_Dish_C|SetmyColour _returnvalue_2 (Variables|Default|GetmyColour)))
        (Variables|/Game/Blueprints/BP_Paint_Dish.BP_Paint_Dish_C|SetinfiniteColourings _returnvalue_2 false)
        (Variables|/Game/Blueprints/BP_Paint_Dish.BP_Paint_Dish_C|SetcolouringsLeft _returnvalue_2 1)
        (bind _returnvalue_3 (Utilities|GetDataTableRow "/Game/Blueprints/DT_Colour_Info.DT_Colour_Info" (Utilities|String|StringToName (Utilities|String|EnumtoString _output_get)))
          (:then
            (bind _returnvalue_4 (Rendering|Material|CreateDynamicMaterialInstance "/Game/Art/Materials/M_Colour.M_Colour" "None" :!class /Script/Engine.KismetMaterialLibrary))
            (Rendering|Material|SetVectorParameterValue _returnvalue_4 "baseColour" (.Colour (Utilities|Struct|BreakST_Colour_Info _returnvalue_3)) :!class /Script/Engine.MaterialInstanceDynamic)
            (Rendering|Material|SetMaterial (Variables|/Game/Blueprints/BP_Paint_Dish.BP_Paint_Dish_C|GetColourant _returnvalue_2) 0 _returnvalue_4)))))
    (elif (Variables|Default|Getthirsty)
      (if (Math|Boolean|NORBoolean (Variables|Default|GetisSlurping) (Variables|Default|GetisDying))
        (|drainColour _asbp_kuutio)))))

(fn ConstructionScript
  ;[1 1 1] Set my colour based off of my enum value.
  (bind _returnvalue (Utilities|GetDataTableRow "/Game/Blueprints/DT_Colour_Info.DT_Colour_Info" (Utilities|String|StringToName (Utilities|String|EnumtoString (Variables|Default|GetmyColour))))
    (:then
      (bind _returnvalue_2 (Rendering|Material|CreateDynamicMaterialInstance "/Game/Art/Materials/M_Colour.M_Colour" "None" :!class /Script/Engine.KismetMaterialLibrary))
      (Rendering|Material|SetVectorParameterValue _returnvalue_2 "baseColour" (.Colour (Utilities|Struct|BreakST_Colour_Info _returnvalue)) :!class /Script/Engine.MaterialInstanceDynamic)
      (Rendering|Material|SetMaterial (Variables|Character|GetMesh) 0 _returnvalue_2)
      ;[1 1 1] Then set my movement speed.
      (Variables|/Script/Engine.CharacterMovementComponent|SetMaxWalkSpeed (Variables|Character|GetCharacterMovement) (Variables|Default|GetmovementSpeed)))))
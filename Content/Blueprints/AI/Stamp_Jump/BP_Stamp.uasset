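; BP_Stamp is a jumping enemy that tries to crush the player and dies, bouncing them upward, when they touch its DamageArea.
; Tick switches between random roaming hops and, while the player is in Range, cooldown-limited leaps toward them or slams from directly above.
; Movement uses timed LaunchCharacter impulses.
; Upward-normal hits deal "Smash" damage, Range toggles alert material and plays sounds, and PlayerCollideDetection halts players, forcing falling ones down.
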(event OnComponentEndOverlap(PlayerCollideDetection)
  (params (OverlappedComponent :type Primitive%20Component%20Object%20Reference) (OtherActor :type Actor%20Object%20Reference) (OtherComp :type Primitive%20Component%20Object%20Reference) (OtherBodyIndex :type Integer))
  (if (Actor|ActorHasTag OtherActor "Player")
    (Variables|Default|SetIsLandedOnPlayer false)))

(event OnComponentEndOverlap(Range)
  (params (OverlappedComponent :type Primitive%20Component%20Object%20Reference) (OtherActor :type Actor%20Object%20Reference) (OtherComp :type Primitive%20Component%20Object%20Reference) (OtherBodyIndex :type Integer))
  (if (Actor|ActorHasTag OtherActor "Player")
    (Variables|Default|SetIsTriggered false)
    (Rendering|Material|SetMaterial (Variables|Character|GetMesh) 0 "/Game/Asset_Packs/Platformer/Materials/M_Cloud.M_Cloud")))

(event OnComponentEndOverlap(PlayerUnderDetection)
  (params (OverlappedComponent :type Primitive%20Component%20Object%20Reference) (OtherActor :type Actor%20Object%20Reference) (OtherComp :type Primitive%20Component%20Object%20Reference) (OtherBodyIndex :type Integer))
  (if (Actor|ActorHasTag OtherActor "Player")
    (Variables|Default|SetOnTopOfPlayer false)))

(event OnComponentBeginOverlap(PlayerUnderDetection)
  (params (OverlappedComponent :type Primitive%20Component%20Object%20Reference) (OtherActor :type Actor%20Object%20Reference) (OtherComp :type Primitive%20Component%20Object%20Reference) (OtherBodyIndex :type Integer) (bFromSweep :type Boolean) (SweepResult :type Hit%20Result%20Structure%20%28by%20ref%29))
  (if (Actor|ActorHasTag OtherActor "Player")
    (Variables|Default|SetOnTopOfPlayer true)))

(event OnComponentBeginOverlap(Range)
  (params (OverlappedComponent :type Primitive%20Component%20Object%20Reference) (OtherActor :type Actor%20Object%20Reference) (OtherComp :type Primitive%20Component%20Object%20Reference) (OtherBodyIndex :type Integer) (bFromSweep :type Boolean) (SweepResult :type Hit%20Result%20Structure%20%28by%20ref%29))
  (bind _returnvalue (Transformation|GetActorLocation))
  (if (Actor|ActorHasTag OtherActor "Player")
    (Variables|Default|SetIsTriggered true)
    (Audio|PlaySoundatLocation "/Game/Audio/SoundForAI/Alert.Alert" _returnvalue "0, 0, 0" 1.0 1.0 0.0 0 0 0)
    (Audio|PlaySoundatLocation "/Game/Audio/SoundForAI/What_are_you_doing_in_my_swamp.What_are_you_doing_in_my_swamp" _returnvalue "0, 0, 0" 1.0 1.0 0.0 0 0 0)
    (Rendering|Material|SetMaterial (Variables|Character|GetMesh) 0 "/Game/Art/Textures/Exclamation_MA.Exclamation_MA")))

(event OnComponentBeginOverlap(DamageArea)
  (params (OverlappedComponent :type Primitive%20Component%20Object%20Reference) (OtherActor :type Actor%20Object%20Reference) (OtherComp :type Primitive%20Component%20Object%20Reference) (OtherBodyIndex :type Integer) (bFromSweep :type Boolean) (SweepResult :type Hit%20Result%20Structure%20%28by%20ref%29))
  (if (Actor|ActorHasTag OtherActor "Player")
    (Components|Movement|StopMovementImmediately (Variables|Character|GetCharacterMovement))
    (bind _asbp_kuutio (Utilities|Casting|CastToBP_Kuutio OtherActor))
    (Character|LaunchCharacter _asbp_kuutio "0, 0,800.000000" false true)
    (Audio|PlaySoundatLocation "/Game/Audio/SoundForAI/Dead.Dead" (Transformation|GetActorLocation) "0, 0, 0" 1.0 1.0 0.0 0 0 0)
    (Actor|DestroyActor)))

(event OnComponentBeginOverlap(PlayerCollideDetection)
  (params (OverlappedComponent :type Primitive%20Component%20Object%20Reference) (OtherActor :type Actor%20Object%20Reference) (OtherComp :type Primitive%20Component%20Object%20Reference) (OtherBodyIndex :type Integer) (bFromSweep :type Boolean) (SweepResult :type Hit%20Result%20Structure%20%28by%20ref%29))
  (if (Actor|ActorHasTag OtherActor "Player")
    (bind _asbp_kuutio (Utilities|Casting|CastToBP_Kuutio OtherActor))
    (Components|Movement|StopMovementImmediately (Variables|/Script/Engine.Character|GetCharacterMovement _asbp_kuutio))
    (if (AI|Components|NavMovement|IsFalling (Variables|/Script/Engine.Character|GetCharacterMovement _asbp_kuutio))
      (Character|LaunchCharacter _asbp_kuutio "0.000000,0.000000,-2000.000000" false false)
      (Variables|Default|SetIsLandedOnPlayer true))))

(event Collision|EventHit
  (params (MyComp :type Primitive%20Component%20Object%20Reference) (Other :type Actor%20Object%20Reference) (OtherComp :type Primitive%20Component%20Object%20Reference) (bSelfMoved :type Boolean) (HitLocation :type Vector :default "0, 0, 0") (HitNormal :type Vector :default "0, 0, 0") (NormalImpulse :type Vector :default "0, 0, 0") (Hit :type Hit%20Result%20Structure%20%28by%20ref%29))
  (if (== Other (Game|GetPlayerCharacter 0))
    (if (> (Math|Vector|DotProduct HitNormal "0, 0,1.000000") 0.9)
      (bind _asbp_kuutio (Utilities|Casting|CastToBP_Kuutio Other))
      (Variables|/Game/Kuutio/BP_Kuutio.BP_Kuutio_C|SetAttack%20By%20 _asbp_kuutio "Smash")
      (Game|Damage|ApplyDamage _asbp_kuutio 3.0 0 0))))

(event EventTick
  (params (DeltaSeconds :type Float%20%28single-precision%29))
  (if (Variables|Default|GetIsTriggered)
    (CallFunction|Triggered)
    (else
      (CallFunction|Roaming))))

(event Custom|Triggered
  (Utilities|FlowControl|Sequence
    (:then_0
      (if (not (AI|Components|NavMovement|IsFalling (Variables|Character|GetCharacterMovement)))
        (if (not (Variables|Default|GetOnTopOfPlayer))
          (if (Variables|Default|GetOffCD)
            (CallFunction|LaunchtoPlayer)
            (Variables|Default|SetOffCD false)
            (Utilities|FlowControl|Delay 0.5)
            (Character|LaunchCharacter "0, 0,-2000.000000" false true)
            (Utilities|FlowControl|Delay (Variables|Default|GetJumpCD))
            (Variables|Default|SetOffCD true)))))
    (:then_1
      (if (Variables|Default|GetOnTopOfPlayer)
        (if (not (AI|Components|NavMovement|IsFalling (Variables|Character|GetCharacterMovement)))
          (Character|LaunchCharacter "0, 0,800.000000" true true)
          (Utilities|FlowControl|Delay 0.5)
          (Character|LaunchCharacter "0, 0,-2000.000000" true true))))))

(event Custom|Roaming
  (if (not (AI|Components|NavMovement|IsFalling (Variables|Character|GetCharacterMovement)))
    (Utilities|FlowControl|Delay 1.0)
    (Character|LaunchCharacter (Math|Vector|MakeVector (Math|Random|RandomFloatinRange -3e+02 3e+02) (Math|Random|RandomFloatinRange -3e+02 3e+02) 8e+02) false true)))

(fn ConstructionScript)

(fn LaunchtoPlayer
  (Character|LaunchCharacter (+ (* (Math|Vector|GetUnitDirection(Vector) (Transformation|GetActorLocation) (Transformation|GetActorLocation (Game|GetPlayerCharacter 0))) (Variables|Default|GetJumpSpeed)) "0, 0,1000.000000") true true))
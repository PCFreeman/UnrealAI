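; BP_Turpentine is a turpentine hazard that strips BP_Kuutio on contact.
; Its Collider plays a sound for any overlapping actor, flags a non-blinking Kuutio as InTurpentine and calls Strip, then clears the flag on exit.
; An optional Cleanup volume, removed in the construction script unless IncludeCleanup is set, respawns a Kuutio that touches it.
; Any other actor touching Cleanup makes the turpentine destroy itself.
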(event OnComponentBeginOverlap(Collider)
  (params (OverlappedComponent :type Primitive%20Component%20Object%20Reference) (OtherActor :type Actor%20Object%20Reference) (OtherComp :type Primitive%20Component%20Object%20Reference) (OtherBodyIndex :type Integer) (bFromSweep :type Boolean) (SweepResult :type Hit%20Result%20Structure%20%28by%20ref%29))
  (Audio|PlaySoundatLocation "/Game/Audio/S_Turpentine.S_Turpentine" (Transformation|GetActorLocation OtherActor) "0, 0, 0" 1.0 1.0 0.0 0 0 0)
  (bind _asbp_kuutio (Utilities|Casting|CastToBP_Kuutio OtherActor))
  (if (not (Variables|/Game/Kuutio/BP_Kuutio.BP_Kuutio_C|Getblinking _asbp_kuutio))
    (Variables|/Game/Kuutio/BP_Kuutio.BP_Kuutio_C|SetinTurpentine _asbp_kuutio true)
    (Default|Strip _asbp_kuutio)))

(event OnComponentBeginOverlap(Cleanup)
  (params (OverlappedComponent :type Primitive%20Component%20Object%20Reference) (OtherActor :type Actor%20Object%20Reference) (OtherComp :type Primitive%20Component%20Object%20Reference) (OtherBodyIndex :type Integer) (bFromSweep :type Boolean) (SweepResult :type Hit%20Result%20Structure%20%28by%20ref%29))
  (bind _asbp_kuutio (Utilities|Casting|CastToBP_Kuutio OtherActor)
    (:then
      (Default|Respawn _asbp_kuutio))
    (:CastFailed
      (Actor|DestroyActor))))

(event OnComponentEndOverlap(Collider)
  (params (OverlappedComponent :type Primitive%20Component%20Object%20Reference) (OtherActor :type Actor%20Object%20Reference) (OtherComp :type Primitive%20Component%20Object%20Reference) (OtherBodyIndex :type Integer))
  (bind _asbp_kuutio (Utilities|Casting|CastToBP_Kuutio OtherActor))
  (Variables|/Game/Kuutio/BP_Kuutio.BP_Kuutio_C|SetinTurpentine _asbp_kuutio false))

(fn ConstructionScript
  (if (not (Variables|Default|GetincludeCleanup))
    (Components|DestroyComponent (Variables|Default|GetCleanup))))
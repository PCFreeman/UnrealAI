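; Actor that moves, rotates and scales a cube between its centre transform and an editable Destination, following a spline and starting on BeginPlay.
; A timeline, rate-scaled by LengthOfTimeline, drives a transform lerp from the centre toward a target built from spline position plus Destination rotation and scale.
; A Delay off the timeline update re-triggers a FlipFlop, alternating play and reverse.
; The construction script places TransformDestination at Destination.
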(event EventBeginPlay
  (bind _spline (Variables|Default|GetSpline))
  (bind _timeline_0 (Variables|Default|GetTimeline_0))
  (bind _destination (Variables|Default|GetDestination))
  (bind _lengthoftimeline (Variables|Default|GetlengthOfTimeline))
  (bind (_location _rotation _scale) (Math|Transform|BreakTransform _destination))
  (bind _returnvalue (/ 1.0 _lengthoftimeline))
  (Utilities|FlowControl|FlipFlop :!label _label
    (:A
      ;[1 1 1] Sets Playback Time
      (Components|Timeline|SetPlayRate _timeline_0 _returnvalue)
      (bind _output (Timeline|Timeline_0 PlayFromStart)
        (:Update
          ;[1 1 1] sets destination point
          (Transformation|SetRelativeTransform (Variables|Default|GetCubeActual) (Math|Transform|Lerp(Transform) (Transformation|GetRelativeTransform (Variables|Default|GetCentre_of_Object)) (Math|Transform|MakeTransform (Spline|GetLocationatDistanceAlongSpline _spline (Math|Float|Lerp 0.0 (Spline|GetSplineLength _spline) _output) "Local") _rotation _scale) _output) false false)
          ;[1 1 1] Delay until reverce
          (Utilities|FlowControl|Delay (+ (Variables|Default|GetlengthOfTimeline) (Variables|Default|Getdelay)))
          (goto _label))))
    (:B
      (Components|Timeline|SetPlayRate _timeline_0 _returnvalue)
      (Timeline|Timeline_0 Reverse))))

(fn ConstructionScript
  (Transformation|SetRelativeTransform (Variables|Default|GetTransformDestination) (Variables|Default|GetDestination) false false))
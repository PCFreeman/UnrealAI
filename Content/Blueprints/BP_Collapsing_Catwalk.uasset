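; BP_Collapsing_Catwalk is a catwalk that collapses when the player character steps on or hits it.
; Overlapping the Collision component plays a crunch warning, then after a short delay plays a crack and enables physics simulation on the Catwalk.
; A player hit on the Catwalk skips the warning and collapses it immediately.
; A shared Triggered flag makes whichever path fires first the only one to run.
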(event OnComponentBeginOverlap(Collision)
  (params (OverlappedComponent :type Primitive%20Component%20Object%20Reference) (OtherActor :type Actor%20Object%20Reference) (OtherComp :type Primitive%20Component%20Object%20Reference) (OtherBodyIndex :type Integer) (bFromSweep :type Boolean) (SweepResult :type Hit%20Result%20Structure%20%28by%20ref%29))
  ;[1 1 1] If overlapped by the character and not already hit with force, begin collapse
  (if (== OtherActor (Game|GetPlayerCharacter 0))
    (Utilities|FlowControl|Delay 0.1)
    (if (not (Variables|Default|Gettriggered))
      (Variables|Default|Settriggered true)
      ;[1 1 1] Play warning sound and wait
      (Audio|PlaySoundatLocation "/Game/Audio/SC_Crunch.SC_Crunch" (Transformation|GetActorLocation) "0, 0, 0" 1.0 1.0 0.0 0 0 0)
      (Utilities|FlowControl|Delay 0.75)
      ;[1 1 1] Then play destroy sound and simulate physics
      (Audio|PlaySoundatLocation "/Game/Audio/S_Crack.S_Crack" (Transformation|GetActorLocation) "0, 0, 0" 1.0 1.0 0.0 0 0 0)
      (Physics|SetSimulatePhysics (Variables|Default|GetCatwalk) true))))

(event OnComponentHit(Catwalk)
  (params (HitComponent :type Primitive%20Component%20Object%20Reference) (OtherActor :type Actor%20Object%20Reference) (OtherComp :type Primitive%20Component%20Object%20Reference) (NormalImpulse :type Vector :default "0, 0, 0") (Hit :type Hit%20Result%20Structure%20%28by%20ref%29))
  ;[1 1 1] If hit with force from player, ignore delay and instantly collapse
  (if (== OtherActor (Game|GetPlayerCharacter 0))
    (if (not (Variables|Default|Gettriggered))
      (Variables|Default|Settriggered true)
      ;[1 1 1] Then play destroy sound and simulate physics
      (Audio|PlaySoundatLocation "/Game/Audio/S_Crack.S_Crack" (Transformation|GetActorLocation) "0, 0, 0" 1.0 1.0 0.0 0 0 0)
      (Physics|SetSimulatePhysics (Variables|Default|GetCatwalk) true))))

(fn ConstructionScript)
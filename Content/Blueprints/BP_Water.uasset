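; BP_Water is a water hazard that clears the player's buffs and resets them to default on contact, unless BP_Kuutio is blinking.
; Any overlap plays a splat sound and optionally prints debug messages.
; An optional Cleanup component, removed in the construction script when disabled, respawns BP_Kuutio on overlap.
; Any other actor entering Cleanup makes the water destroy itself.
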(event OnComponentBeginOverlap(Cleanup)
  (params (OverlappedComponent :type Primitive%20Component%20Object%20Reference) (OtherActor :type Actor%20Object%20Reference) (OtherComp :type Primitive%20Component%20Object%20Reference) (OtherBodyIndex :type Integer) (bFromSweep :type Boolean) (SweepResult :type Hit%20Result%20Structure%20%28by%20ref%29))
  (bind _asbp_kuutio (Utilities|Casting|CastToBP_Kuutio OtherActor)
    (:then
      (Default|Respawn _asbp_kuutio))
    (:CastFailed
      (Actor|DestroyActor))))

(event Collision|EventActorBeginOverlap
  (params (OtherActor :type Actor%20Object%20Reference))
  ;[1 1 1] Collision
  (Audio|PlaySoundatLocation "/Game/Audio/S_PaintDish.S_PaintDish" (Transformation|GetActorLocation OtherActor) "0, 0, 0" 1.0 1.0 0.0 0 0 0)
  ;;[1 1 1] Confirm contact if messages enabled
  (if (Variables|Default|GetdisableMessages)
    _
    (else
      (Development|PrintString (Utilities|String|Append (Utilities|GetDisplayName OtherActor) " Contacted " "Water"))))
  ;;[1 1 1] Continue execution if isPlayer, and print appropriate names if messages on
  (if (== OtherActor (Game|GetPlayerCharacter 0))
    (if (Variables|Default|GetdisableMessages)
      _
      (else
        (Development|PrintString "Match")))
    (bind _asbp_kuutio (Utilities|Casting|CastToBP_Kuutio OtherActor))
    (if (not (Variables|/Game/Kuutio/BP_Kuutio.BP_Kuutio_C|Getblinking _asbp_kuutio))
      (Default|TerminateBuffs _asbp_kuutio)
      (Default|ResettoDefault _asbp_kuutio))
    (elif (not (Variables|Default|GetdisableMessages))
      (Development|PrintString (Utilities|GetDisplayName OtherActor)))))

(fn ConstructionScript
  (if (not (Variables|Default|GetincludeCleanup))
    (Components|DestroyComponent (Variables|Default|GetCleanup))))
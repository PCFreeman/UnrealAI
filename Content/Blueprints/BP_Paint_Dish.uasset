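; Paint dish that colours the player's BP_Kuutio on overlap, setting its active colour and refilling that ability's remaining amount.
; The construction script looks up MyColour in DT_Colour_Info and tints the Colourant through a dynamic material instance.
; Pawn overlap is enabled shortly after BeginPlay; contact clears buffs and plays sound and a brief effect burst behind a Colouring lock.
; Unless colourings are infinite, each use decrements a counter and the dish destroys itself when depleted.
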(event EventBeginPlay
  ;[1 1 1] Prevent the player from overlapping the paintdish before it receives its colouring.
  (Utilities|FlowControl|Delay 1.0)
  (Collision|SetCollisionResponsetoChannel (Variables|Default|GetColourant) "ECC_Pawn" "ECR_Overlap"))

(event OnComponentBeginOverlap(Colourant)
  (params (OverlappedComponent :type Primitive%20Component%20Object%20Reference) (OtherActor :type Actor%20Object%20Reference) (OtherComp :type Primitive%20Component%20Object%20Reference) (OtherBodyIndex :type Integer) (bFromSweep :type Boolean) (SweepResult :type Hit%20Result%20Structure%20%28by%20ref%29))
  (bind _colouringsleft (Variables|Colouring|GetcolouringsLeft))
  (if (and (not (Variables|Default|Getcolouring)) (Actor|ActorHasTag OtherActor "Player"))
    (Audio|PlaySound2D "/Game/Audio/S_PaintDish.S_PaintDish" 1.0 1.0 0.0 0 0)
    (bind _asbp_kuutio (Utilities|Casting|CastToBP_Kuutio OtherActor))
    (bind _output_get (Variables|Default|Setcolouring true))
    (Variables|/Game/Kuutio/BP_Kuutio.BP_Kuutio_C|Setcolouring _asbp_kuutio _output_get)
    (Default|TerminateBuffs _asbp_kuutio)
    ;[1 1 1] Update appropriate side's colour
    (Variables|/Game/Kuutio/BP_Kuutio.BP_Kuutio_C|SetactiveColour _asbp_kuutio (Variables|Colouring|GetmyColour))
    ;[1 1 1] Then refresh ability amount remaining
    (Variables|/Game/Kuutio/BP_Kuutio.BP_Kuutio_C|SetactiveAbilityRemaining _asbp_kuutio (Variables|/Game/Kuutio/BP_Kuutio.BP_Kuutio_C|GetmaxAbilityRemaining _asbp_kuutio))
    ;[1 1 1] Then update visuals and make visual feedback via 'spurt' of appropriate colour
    (bind _particleref (Default|UpdateEffects _asbp_kuutio))
    (Components|Activation|Activate _particleref false)
    (Utilities|FlowControl|Delay 0.4)
    (Components|Activation|Deactivate _particleref)
    (bind _output_get_2 (Variables|Default|Setcolouring false))
    (Variables|/Game/Kuutio/BP_Kuutio.BP_Kuutio_C|Setcolouring _asbp_kuutio _output_get_2)
    ;[1 1 1] Then, if I don't have infinite colourings...
    (if (not (Variables|Colouring|GetinfiniteColourings))
      ;[1 1 1] Subtract my colouringsLeft, and destroy self after hitting 0
      (Math|Integer|DecrementInt _colouringsleft
        (:%20%20
          (if (<= _colouringsleft 0)
            (Actor|DestroyActor)))))))

(fn ConstructionScript
  (bind _mycolour (Variables|Colouring|GetmyColour))
  (bind _returnvalue (Utilities|String|EnumtoString _mycolour))
  (bind _returnvalue_2 (Utilities|String|StringToName _returnvalue))
  ;[1 1 1] Return DT row based off of 'MyColour' enum value
  (Physics|SetSimulatePhysics (Variables|Default|GetPaintDishBase) (Variables|Default|Getmovable))
  (bind _returnvalue_3 (Utilities|GetDataTableRow "/Game/Blueprints/DT_Colour_Info.DT_Colour_Info" _returnvalue_2)
    (:then
      ;[1 1 1] Print myColour if messages enabled
      (if (Variables|Default|GetdisableMessages)
        _
        (else
          (Development|PrintString (Utilities|String|ToString(Name) _returnvalue_2))))
      ;[1 1 1] Create dynamic instance with corresponding DT colour value, and set my mesh to that colour.
      (bind _returnvalue_4 (Rendering|Material|CreateDynamicMaterialInstance "/Game/Art/Materials/M_Colour.M_Colour" "None" :!class /Script/Engine.KismetMaterialLibrary))
      (Rendering|Material|SetVectorParameterValue _returnvalue_4 "baseColour" (.Colour (Utilities|Struct|BreakST_Colour_Info _returnvalue_3)) :!class /Script/Engine.MaterialInstanceDynamic)
      (Rendering|Material|SetMaterial (Variables|Default|GetColourant) 0 _returnvalue_4))))
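; Collectible coin actor from a platformer asset pack that ends the game when picked up.
; It spins on Tick with a fixed local rotation that is not scaled by delta time.
; When the player character overlaps it, it destroys its mesh and plays a collect sound, then after a short delay quits the game and destroys itself.
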(event EventTick
  (params (DeltaSeconds :type Float%20%28single-precision%29))
  ;[1 1 1] Rotate in place
  (Transformation|AddActorLocalRotation "0,5.000000, 0" false false))

(event Collision|EventActorBeginOverlap
  (params (OtherActor :type Actor%20Object%20Reference))
  ;[1 1 1] On contact with other actor
  ;;[1 1 1] If player
  (if (== OtherActor (Game|GetPlayerCharacter 0))
    ;;[1 1 1] Destroy collectible and play sound
    (Components|DestroyComponent (Variables|Default|GetStaticMesh))
    (Audio|PlaySoundatLocation "/Game/Audio/S_Collectible.S_Collectible" (Transformation|GetActorLocation) "0, 0, 0" 1.0 1.0 0.0 0 0 0)
    ;;[1 1 1] Then quit game after delay
    (Utilities|FlowControl|Delay 2.0)
    (Game|QuitGame (Game|GetPlayerController 0) "Quit" false)
    (Actor|DestroyActor)))

(fn ConstructionScript)